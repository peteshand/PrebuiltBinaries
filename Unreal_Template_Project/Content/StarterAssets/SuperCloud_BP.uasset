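; SuperCloud_BP is a touch-interactive cloud actor that plays a one-shot animation when tapped.
; When a touch ends on ActiveArea and passes CheckIfTap, it hides the Tooltip and plays SuperCloud_Anim on SuperCloud.
; The Check if Tap graph stores the Touch1 screen position at touch begin.
; Its comparison of that start point with the current touch position is left unconnected.
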(event OnInputTouchEnd(ActiveArea)
  (params (FingerIndex :type ETouchIndex%20Enum :default "Touch1") (TouchedComponent :type Primitive%20Component%20Object%20Reference))
  (if (|CheckifTap FingerIndex)
    (Rendering|SetVisibility (Variables|Default|GetTooltip) false false)
    (Components|Animation|PlayAnimation (Variables|Default|GetSuperCloud) "/Game/StarterAssets/Meshes/SuperCloud_Anim.SuperCloud_Anim" false)))

(fn ConstructionScript)

(event EventActorOnInputTouchBegin
  (params (FingerIndex :type ETouchIndex%20Enum :default "Touch1"))
  (bind _returnvalue (Game|GetPlayerController 0))
  (bind (_locationx _locationy) (Class|PlayerController|GetInputTouchState _returnvalue "Touch1"))
  (Variables|Default|SetTouchStart (Math|Vector2D|MakeVector2D _locationx _locationy)))