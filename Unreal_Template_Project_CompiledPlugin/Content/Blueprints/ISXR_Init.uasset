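; ISXR_Init is a level initializer actor for a cloud AR/XR streaming app that runs startup console commands and spawns mode-switch and side-channel actors.
; A received asset ID is saved in the GameInstance for restoring on BeginPlay, and serves example logic that hides the SuperCloud or opens a level named before the colon.
; It also relays URL redirects, offers debug console commands, and shows an AR bounding box guide in construction.
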(event Custom|RedirectToUrl
  (params (URL :type String))
  ;[0 0 0] DO NOT EDIT
  ;;[0 0 0] URL Redirect
  (Default|CallRedirecttoUrlDispatch URL))

(event Custom|GetCloudARAssetID
  (params (CloudARAssetID :type String))
  ;[0 0 0] Asset ID
  (bind _asasset_idvar_global (Utilities|Casting|CastToAssetIDVar_Global (Game|GetGameInstance))
    (:then
      (Variables|/Game/Blueprints/AssetIDVar_Global.AssetIDVar_Global_C|SetInitialCloudARAssetID _asasset_idvar_global CloudARAssetID))
    (:CastFailed
      _))
  (bind _output_get (Variables|Default|SetCloudARAssetID CloudARAssetID))
  ;[0.06236 0.09896 0.08163] Example A: Switch 3D Cloud Asset with Asset ID from URL
  (bind _returnvalue (Actor|GetActorOfClass "/Game/StarterAssets/SuperCloud_BP.SuperCloud_BP_C"))
  (if (Utilities|Enum|Equal(Enum) _output_get "Super_Cloud_Particles")
    (Rendering|ToggleVisibility (Variables|/Game/StarterAssets/SuperCloud_BP.SuperCloud_BP_C|GetSuperCloud _returnvalue) false))
  ;[0.06236 0.09896 0.08163] Example B: Load Demos with Asset ID from URL
  (if (.ReturnValue (Utilities|String|Split (Variables|Default|GetCloudARAssetID) ":"))
    (Game|OpenLevel(byName) (Utilities|String|StringToName (.LeftS (Utilities|String|Split (Variables|Default|GetCloudARAssetID) ":"))) false)))

(event Custom|ToggleConsoleCommands
  ;[0 0 0] DO NOT EDIT
  ;;[0 0 0] Console Commands
  (CallFunction|ConsoleCommand))

(event EventBeginPlay
  ;[0 0 0] DO NOT EDIT
  ;;[0 0 0] Run init commands
  (for _array_element (Variables|Default|GetInitCommands)
    (Development|ExecuteConsoleCommand _array_element 0))
  (Development|ExecuteConsoleCommand (Variables|Default|GetCameraControl) 0)
  ;;[0 0 0] Load Blueprints
  (Game|SpawnActorfromClass (Variables|Default|GetModeSwitch_class) (Math|Transform|MakeTransform "0, 0, 0" "0, 0, 0" "1.000000,1.000000,1.000000") "Undefined" "OverrideRootScale" 0 0)
  (Game|SpawnActorfromClass (Variables|Default|GetSideChannel_class) (Math|Transform|MakeTransform "0, 0, 0" "0, 0, 0" "1.000000,1.000000,1.000000") "Undefined" "SelectDefaultAtRuntime" 0 0)
  ;;[0 0 0] Get Global Asset ID
  (if (Utilities|Enum|Equal(Enum) (Variables|Default|GetCloudARAssetID) "Default:Session_ID:000")
    (bind _asasset_idvar_global (Utilities|Casting|CastToAssetIDVar_Global (Game|GetGameInstance)))
    (Variables|Default|SetCloudARAssetID (Variables|/Game/Blueprints/AssetIDVar_Global.AssetIDVar_Global_C|GetInitialCloudARAssetID _asasset_idvar_global))))

(fn ConstructionScript
  (bind _boundingbox (Variables|Default|GetBoundingBox))
  (bind _boundingboxguide (Variables|Default|GetBoundingBoxGuide))
  (if (Variables|ARMode|GetAR%20ModeEnabled)
    (Rendering|SetVisibility _boundingbox true true)
    (Transformation|SetWorldScale3D _boundingboxguide (Variables|ARMode|GetBoundingBoxSize))
    (Transformation|SetWorldLocation _boundingboxguide "0, 0, 0" false false)
    (else
      (Rendering|SetVisibility _boundingbox false true))))

(fn ConsoleCommand
  (for _array_element (Variables|DebugMode|GetDebugStatsCommands)
    (Development|ExecuteConsoleCommand _array_element 0))
  (Development|ExecuteConsoleCommand "r.ScreenPercentage 100" 0)
  (Development|ExecuteConsoleCommand "r.C9.RenderDebugMessages 1" 0)
  (return 0))